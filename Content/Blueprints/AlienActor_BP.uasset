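; Alien actor Blueprint that exposes events for changing the look and animation of an alien skeletal mesh.
; Events swap the mesh, apply the stored material to the first slot, or pick the Generic or Enthusiast AnimBP by index, defaulting to Generic.
; PlayAnimMontage plays an entry from a montage array by index.
; ChangeAnimMontage, BeginPlay and the construction script are empty, and leftover idle/confused state and input nodes are disconnected.
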(event Custom|SetMesh
  (params (Mesh :type Skeletal%20Mesh%20Object%20Reference))
  ;[1 1 1] Set Mesh
  (Class|SkinnedMeshComponent|SetSkeletalMesh (Variables|Default|GetAlien_SkeletalMesh) Mesh true))

(event Custom|SetTexture
  ;[1 1 1] Set Texture
  (Rendering|Material|SetMaterial (Variables|Default|GetAlien_SkeletalMesh) 0 (Variables|Default|GetAlienMaterial)))

(event Custom|SetAnimBP
  (params (AnimBP :type Integer))
  (bind _alien_skeletalmesh (Variables|Default|GetAlien_SkeletalMesh))
  ;[1 1 1] Set AnimBP
  (switch int AnimBP
    (:Default
      (Class|SkeletalMeshComponent|SetAnimClass _alien_skeletalmesh "/Game/Assets/3D/Yoppoppo_Generic/AnimationBP_Generic.AnimationBP_Generic_C" :!label _label))
    (:0
      (goto _label))
    (:1
      (Class|SkeletalMeshComponent|SetAnimClass _alien_skeletalmesh "/Game/Assets/3D/Yoppoppo_Enthusiast/AnimationBP_Enthusiast.AnimationBP_Enthusiast_C"))))

(event Custom|ChangeAnimMontage
  (params (Anim :type Integer)))

(event Custom|PlayAnimMontage
  (params (Anim :type Integer))
  ;[1 1 1] Play Anim Montage
  (bind _output_get (Variables|Default|SetCurrentAnimMontage (Utilities|Array|Get(acopy) (Variables|Default|GetAnimMontageArray) Anim)))
  (Animation|Montage|PlayMontage (Variables|Default|GetAlien_SkeletalMesh) _output_get))

(event EventBeginPlay
  ;[1 1 1] Testing
)

(event Input|KeyboardEvents|F
  (params (Key :type Key%20Structure :default "None"))
  ;[1 1 1] Testing
)

(fn ConstructionScript)