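; AlienManager_BP manages level progression by configuring the level's AlienActor_BP from data tables.
; NextLevel reads the AlienList row named by LevelCount, loads that alien's phase table, then sets mesh and integer-indexed AnimBP after a delay.
; GetNewPhaseData reads numbered phase rows; a missing row resets the phase, increments the level and calls NextLevel.
; GetOpeningOutput exposes the current alien's starting output.
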(event Custom|NextLevel
  (bind _aliens (Variables|Default|Getaliens))
  (bind _currentalienbp (Variables|Default|GetCurrentAlienBP))
  (bind (_alienmesh _alienanimbp _aliendata) (Utilities|Struct|BreakAlienList _aliens))
  (bind _output (Utilities|ResolveSoftReference _aliendata))
  (bind _returnvalue (Utilities|GetDataTableRow "/Game/Assets/AlienDatatables/AlienList.AlienList" (Utilities|String|StringToName (Utilities|String|ToString(Integer) (Variables|Default|GetLevelCount))))
    (:then
      (Class|AlienManager|SetAlien _returnvalue)
      (Variables|Default|SetCurrentAlienDataTable _output)
      (CallFunction|GetNewPhaseData _output (Variables|Default|GetphaseCount))
      (bind _outrownames (DataTable|GetDataTableRowNames _output))
      (Variables|Default|SetmaxPhases (Utilities|Array|Length _outrownames))
      (Utilities|FlowControl|Delay 2.0)
      (Default|SetMesh _currentalienbp (Utilities|ResolveSoftReference _alienmesh))
      (Default|SetAnimBP _currentalienbp) ; Use an Int to get the right AnimBP rather than referencing the AnimBP file directly
    )))

(event EventBeginPlay
  (bind _returnvalue (Actor|GetActorOfClass "/Game/Blueprints/AlienActor_BP.AlienActor_BP_C"))
  (Variables|Default|SetCurrentAlienBP _returnvalue)
  (CallFunction|NextLevel))

(event EventTick
  (params (DeltaSeconds :type Float%20%28single-precision%29)))

(fn ConstructionScript)

(fn GetNewPhaseData
  (params (DataTable :type Data%20Table%20Object%20Reference) (CurrentPhase :type Integer))
  (bind _returnvalue (Utilities|GetDataTableRow DataTable (Utilities|String|StringToName (Utilities|String|ToString(Integer) CurrentPhase)))
    (:then
      (Class|AlienManager|SetupLevelPhase _returnvalue)
      (return true))
    (:RowNotFound
      (Variables|Default|SetphaseCount 1)
      (bind _result (Math|Integer|IncrementInt (Variables|Default|GetLevelCount))
        (:%20%20
          (Variables|Default|SetLevelCount _result)
          (CallFunction|NextLevel)
          (return false))))))

(fn BreakData
  (params (Row :type Alien%20Data%20Structure%20%28by%20ref%29))
  (Class|AlienManager|SetupLevelPhase Row))

(fn GetOpeningOutput
  (return (.startingOutput (Utilities|Struct|BreakAlienList (Variables|Default|Getaliens)))))