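; PlayerPawn_BP is the player pawn that sets up the game's UI and handles basic keyboard input.
; On BeginPlay it creates the GameplayHUD and Intro widgets, adds both to the viewport, and caches a reference to the AlienActor_BP in the level.
; Tab and Left Ctrl both call SwapModes on the HUD, while Escape quits the game.
; An unconnected montage call on the alien's mesh never runs.
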(event EventBeginPlay
  (bind _returnvalue (UserInterface|CreateWidget "/Game/HUD/GameplayHUD.GameplayHUD_C" 0 "Default Alien Reply" 0))
  (bind _output_get (Variables|Default|SetHUD%20Reference _returnvalue))
  (UserInterface|Viewport|AddtoViewport _output_get 0)
  (bind _returnvalue_2 (Actor|GetActorOfClass "/Game/Blueprints/AlienActor_BP.AlienActor_BP_C"))
  (Variables|Default|SetAlienRef _returnvalue_2)
  (bind _returnvalue_3 (UserInterface|CreateWidget "/Game/HUD/Intro.Intro_C"))
  (UserInterface|Viewport|AddtoViewport _returnvalue_3 0))

(event Collision|EventActorBeginOverlap
  (params (OtherActor :type Actor%20Object%20Reference)))

(event EventTick
  (params (DeltaSeconds :type Float%20%28single-precision%29)))

(event Input|KeyboardEvents|Tab
  (params (Key :type Key%20Structure :default "None"))
  (:Pressed
    (Default|SwapModes (Variables|Default|GetHUD%20Reference))))

(event Input|KeyboardEvents|LeftCtrl
  (params (Key :type Key%20Structure :default "None"))
  (:Pressed
    (Default|SwapModes (Variables|Default|GetHUD%20Reference))))

(event Input|KeyboardEvents|Escape
  (params (Key :type Key%20Structure :default "None"))
  (:Pressed
    (Game|QuitGame 0 "Quit" false)))

(fn ConstructionScript)